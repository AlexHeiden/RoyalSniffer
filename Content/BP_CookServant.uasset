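; BP_CookServant is a cook servant actor with a randomly coloured skeletal mesh that disappears when the game mode flags probable poison.
; BeginPlay sets the mesh materials' Color parameter to a random colour twice, the second overriding the first, then caches BP_FirstPersonGameMode.
; Tick polls that game mode's ProbablyPoison flag and destroys the actor once it is true.
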(event EventBeginPlay
  (bind _skeletalmesh (Variables|Default|GetSkeletalMesh))
  (Utilities|FlowControl|Sequence
    (:then_0
      (bind _output_get (Variables|Default|SetRandomColor1 (Utilities|Struct|MakeLinearColor (Math|Random|RandomFloatinRange 0.0 1.0) (Math|Random|RandomFloatinRange 0.0 1.0) (Math|Random|RandomFloatinRange 0.0 1.0) 1.0)))
      (Rendering|Material|SetColorParameterValueonMaterials _skeletalmesh "Color" _output_get)
      (bind _output_get_2 (Variables|Default|SetRandomColor2 (Utilities|Struct|MakeLinearColor (Math|Random|RandomFloatinRange 0.0 1.0) (Math|Random|RandomFloatinRange 0.0 1.0) (Math|Random|RandomFloatinRange 0.0 1.0) 1.0)))
      (Rendering|Material|SetColorParameterValueonMaterials _skeletalmesh "Color" _output_get_2))
    (:then_1
      (bind _asbp_first_person_game_mode (Utilities|Casting|CastToBP_FirstPersonGameMode (Game|GetGameMode))))))

(event EventTick
  (params (DeltaSeconds :type Float%20%28single-precision%29))
  (if (Variables|/Game/FirstPerson/Blueprints/BP_FirstPersonGameMode.BP_FirstPersonGameMode_C|GetProbablyPoison (stale EventBeginPlay _asbp_first_person_game_mode))
    (Actor|DestroyActor)))

(fn ConstructionScript)