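; BP_Food is a food actor with a Niagara effect and movement added at runtime.
; On BeginPlay it randomly attempts a Cone static mesh override on the effect with an empty variable name, then caches the first-person character and adds an InterpToMovement component.
; Tick polls the character's ToKing flag, adding another movement component and clearing the shared flag when set.
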(event EventBeginPlay
  (if (Math|Random|RandomBool)
    _
    (else
      (Class|NiagaraFunctionLibrary|OverrideSystemUserVariableStaticMesh (Variables|Default|GetNiagara) "" "/Engine/BasicShapes/Cone.Cone")))
  (bind _asbp_first_person_character (Utilities|Casting|CastToBP_FirstPersonCharacter (Game|GetPlayerCharacter 0)))
  (AddComponent|AddInterptoMovementComponent))

(event EventTick
  (params (DeltaSeconds :type Float%20%28single-precision%29))
  (if (Variables|/Game/FirstPerson/Blueprints/BP_FirstPersonCharacter.BP_FirstPersonCharacter_C|GetToKing (stale EventBeginPlay _asbp_first_person_character))
    (AddComponent|AddInterptoMovementComponent)
    (Variables|/Game/FirstPerson/Blueprints/BP_FirstPersonCharacter.BP_FirstPersonCharacter_C|SetToKing (stale EventBeginPlay _asbp_first_person_character) false)))

(fn ConstructionScript)